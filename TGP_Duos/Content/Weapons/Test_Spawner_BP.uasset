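; Test item spawner that shows a pickup with a blue spotlight and a player-facing text label.
; Tick toggles visibility from HasItem, updates the label or countdown, and respawns the item once RespawnTime reaches its maximum.
; FirstPersonCharacter overlap only clears HasItem, granting nothing.
; The timer resets on spawn, not pickup, so a late pickup can respawn immediately.
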(event `self.ReceiveBeginPlay`)

(event `self.ReceiveTick`
  (params (DeltaSeconds :type "Float (single-precision)"))
  (bind _hasitem (`self.hasItem`))
  (`self.UpdateText`)
  (`SceneComponent.SetVisibility` (`self.Spawn Location`) _hasitem false)
  (`SceneComponent.SetVisibility` (`self.SpotLight`) _hasitem false)
  (if (and (== (`self.hasItem`) (`KismetMathLibrary.Conv_IntToBool` 0)) (>= (`self.respawnTime`) (`self.respawnTimeMax`)))
    (`self.SpawnItem`)
    (set `self.respawnTime` 0.0)
    (else
      (set `self.respawnTime` (+ (`self.respawnTime`) DeltaSeconds)))))

(event `self.Spawn Location.OnComponentBeginOverlap`
  (params (OverlappedComponent :type "PrimitiveComponent Object Reference") (OtherActor :type "Actor Object Reference") (OtherComp :type "PrimitiveComponent Object Reference") (OtherBodyIndex :type Integer) (bFromSweep :type Boolean) (SweepResult :type "HitResult Structure (by ref)"))
  (cast `/Game/FirstPersonCPP/Blueprints/FirstPersonCharacter` OtherActor)
  (if (== (`self.hasItem`) true)
    (`self.PickupItem`)))

(fn `PickupItem`
  (set `self.hasItem` false))

(fn `SpawnItem`
  (`LightComponent.SetLightColor` (`self.SpotLight`) (struct :`R` 0.285414 :`G` 0.29348 :`B` 1.0 :`A` 1.0) true)
  (set `self.hasItem` true))

(fn `UpdateText`
  (`SceneComponent.K2_SetWorldRotation` (`self.TextRender`) (`KismetMathLibrary.FindLookAtRotation` (`SceneComponent.K2_GetComponentLocation` (`self.TextRender`)) (`self.K2_GetActorLocation` (`GameplayStatics.GetPlayerPawn` 0))) false false)
  (if (`self.hasItem`)
    (`TextRenderComponent.K2_SetText` (`self.TextRender`) (`|FormatText` "Item"))
    (else
      (`TextRenderComponent.K2_SetText` (`self.TextRender`) (`KismetTextLibrary.Conv_StringToText` (`KismetStringLibrary.Conv_IntToString` (`KismetMathLibrary.FTrunc` (- (`self.respawnTimeMax`) (`self.respawnTime`)))))))))

(fn `UserConstructionScript`)