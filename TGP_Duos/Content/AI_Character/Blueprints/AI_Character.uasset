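; AI character Blueprint that takes damage and respawns by teleporting when its health runs out.
; The HealthInterfaceComponent event subtracts damage from Health.
; At zero or below, it moves the actor to a random navigable point within a radius on the first RecastNavMesh found, raised on Z, then resets Health and increments its own Kills counter.
; The construction script and NewFunction_0 are empty.
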(event `/Game/FirstPersonCPP/Blueprints/HealthInterface.HealthInterfaceComponent`
  (params (Damage :type "Float (single-precision)"))
  (bind _health (`self.Health`))
  (set `self.Health` (- _health Damage))
  (bind _outactors (`GameplayStatics.GetAllActorsOfClass` "/Script/NavigationSystem.RecastNavMesh"))
  (if (<= _health 0.0)
    (`self.K2_SetActorLocation` (`KismetMathLibrary.MakeVector` (.x (`NavigationSystemV1.K2_GetRandomLocationInNavigableRadius` (`self.K2_GetActorLocation`) 10000.0 (`|GetArrayItem` _outactors) null)) (.y (`NavigationSystemV1.K2_GetRandomLocationInNavigableRadius` (`self.K2_GetActorLocation`) 10000.0 (`|GetArrayItem` _outactors) null)) (+ (.z (`NavigationSystemV1.K2_GetRandomLocationInNavigableRadius` (`self.K2_GetActorLocation`) 10000.0 (`|GetArrayItem` _outactors) null)) 100.0)))
    (set `self.Health` 100.0)
    (set `self.Kills` (+ (`self.Kills`) 1))))

(fn `NewFunction_0`)

(fn `UserConstructionScript`)